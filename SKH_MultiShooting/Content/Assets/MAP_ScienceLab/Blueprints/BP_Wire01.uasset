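; BP_Wire01 is a construction-script spline tool that builds configurable wires from spline mesh components.
; SplineMeshVar selects either one segment per pair of spline points or evenly spaced segments along the spline length, with scaled direction tangents.
; WireVar picks one of six segment variants, three using a second material slot.
; Each segment gets uniform thickness and dynamic MI_Wire instances driven by color, dirt, specular, roughness and texture-set variables.
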(fn ConstructionScript
  (|Wire))