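; BP_Death2 is a death effect actor that plays a death animation, then dissolves its skeletal mesh with Niagara particles.
; On BeginPlay, after a delay, it plays a random montage-free death animation (only the first three of five options are reachable) and disables collision.
; After a second delay, it attaches the Niagara system, swaps three material slots to a dissolve material, and a timeline drives their dissolve amount and emissive color.
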(event EventBeginPlay
  (bind _sk_manq (Variables|Default|GetSK_ManQ))
  (bind _dissolvemat (Variables|Default|GetDissolveMat))
  (Utilities|FlowControl|Delay (Variables|Default|GetDelay))
  (Components|Animation|PlayAnimation (Variables|Default|GetSK_ManQ) (Utilities|Select :Index (Math|Random|RandomIntegerinRange 0 2) :Option%200 "/Game/Assets/EFFECT_NiagaraDeathEffects/Demo/Mannequin/Animations/Flying_Back_Death_mixamo_com.Flying_Back_Death_mixamo_com" :Option%201 "/Game/Assets/EFFECT_NiagaraDeathEffects/Demo/Mannequin/Animations/Standing_Death_Left_02.Standing_Death_Left_02" :Option%202 "/Game/Assets/EFFECT_NiagaraDeathEffects/Demo/Mannequin/Animations/Standing_Death_Right_02.Standing_Death_Right_02" :Option%203 "/Game/Assets/EFFECT_NiagaraDeathEffects/Demo/Mannequin/Animations/Standing_React_Death_Backward_mixamo_com.Standing_React_Death_Backward_mixamo_com" :Option%204 "/Game/Assets/EFFECT_NiagaraDeathEffects/Demo/Mannequin/Animations/Standing_React_Death_Forward_mixamo_com.Standing_React_Death_Forward_mixamo_com") false)
  (Collision|SetCollisionEnabled (Variables|Default|GetSK_ManQ) "NoCollision")
  (Utilities|FlowControl|Delay (Variables|Default|GetNextDelay))
  (Niagara|SpawnSystemAttached (Variables|Default|GetNiagaraDeath) (Variables|Default|GetSK_ManQ) "None" "0, 0, 0" "0, 0, 0" "KeepRelativeOffset" false)
  (Utilities|FlowControl|Sequence
    (:then_0
      (Rendering|Material|SetMaterial _sk_manq 0 _dissolvemat)
      (bind _diss (Timeline|Dissolveation PlayFromStart)
        (:Update
          (CallFunction|DissoleMatParam _sk_manq _diss))))
    (:then_1
      (Rendering|Material|SetMaterial (Variables|Default|GetSK_ManQ) 1 _dissolvemat)
      (Timeline|Dissolveation PlayFromStart))
    (:then_2
      (Rendering|Material|SetMaterial (Variables|Default|GetSK_ManQ) 2 _dissolvemat)
      (Timeline|Dissolveation PlayFromStart))))

(fn ConstructionScript)

(fn DissoleMatParam
  (params (self2 :type Mesh%20Component%20Object%20Reference) (AmountParameterValue :type Float%20%28double-precision%29))
  (Rendering|Material|SetScalarParameterValueonMaterials self2 "Dissolve" AmountParameterValue)
  (Rendering|Material|SetVectorParameterValueonMaterials self2 "Emm color" (Math|Conversions|ToVector(LinearColor) (Variables|Default|GetColor))))