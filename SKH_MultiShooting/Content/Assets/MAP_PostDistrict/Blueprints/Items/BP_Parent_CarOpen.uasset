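; Parent Blueprint for openable car props in four body types (hatchback, pickup, station wagon, ambulance), handling their body paint.
; The construction script runs ConstructCar, which applies one dynamic material instance, chosen by car type and clean or regular version, across the root's child components.
; Paint is random from a palette or manually set, and LOCKVALUES freezes it.
; RandomGenerator, a variant that also randomizes leaves and damage, is not called here.
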(event EventBeginPlay)

(event Collision|EventActorBeginOverlap
  (params (OtherActor :type Actor%20Object%20Reference)))

(event EventTick
  (params (DeltaSeconds :type Float%20%28single-precision%29)))

(fn ConstructionScript
  (CallFunction|ConstructCar (Variables|1.MasterControl|GetRUN_SCRIPT)))

(fn RandomGenerator
  (bind _carcolorpalette (Variables|4.Colors|GetCarColorPalette))
  (bind _defaultsceneroot (Variables|Default|GetDefaultSceneRoot))
  (bind _cartype (Variables|3.MainControl|GetCarType))
  (bind _children (Components|GetChildrenComponents _defaultsceneroot false))
  ;[1 1 1] Create Material Instance
  (bind _as프리미티브_컴포넌트 (Utilities|Casting|CastToPrimitiveComponent (Utilities|Array|Get(acopy) _children 1)))
  (bind _returnvalue (Rendering|Material|CreateDynamicMaterialInstance _as프리미티브_컴포넌트 0 (select (Variables|3.MainControl|GetCleanVersion) (Utilities|Select :Index _cartype :NewEnumerator0 "/Game/Assets/MAP_PostDistrict/Materials/Vehicles/MI_Hatchback_Clean.MI_Hatchback_Clean" :NewEnumerator1 "/Game/Assets/MAP_PostDistrict/Materials/Vehicles/MI_Pickup_Clean.MI_Pickup_Clean" :NewEnumerator2 "/Game/Assets/MAP_PostDistrict/Materials/Vehicles/MI_Wagon_Clean.MI_Wagon_Clean" :NewEnumerator3 "/Game/Assets/MAP_PostDistrict/Materials/Vehicles/MI_Ambulance_Clean.MI_Ambulance_Clean") (Utilities|Select :Index _cartype :NewEnumerator0 "/Game/Assets/MAP_PostDistrict/Materials/Vehicles/MI_Hatchback.MI_Hatchback" :NewEnumerator1 "/Game/Assets/MAP_PostDistrict/Materials/Vehicles/MI_Pickup.MI_Pickup" :NewEnumerator2 "/Game/Assets/MAP_PostDistrict/Materials/Vehicles/MI_Wagon.MI_Wagon" :NewEnumerator3 "/Game/Assets/MAP_PostDistrict/Materials/Vehicles/MI_Ambulance.MI_Ambulance")) "None" :!class /Script/Engine.PrimitiveComponent))
  (Variables|Default|SetCarBodyMatInst _returnvalue)
  ;[1 1 1] Assign Material Instance
  (for _array_element _children
    (bind _as프리미티브_컴포넌트_2 (Utilities|Casting|CastToPrimitiveComponent _array_element))
    (Rendering|Material|SetMaterial _as프리미티브_컴포넌트_2 0 (Variables|Default|GetCarBodyMatInst)))
  (if (Variables|2.RandomControl|GetRandomColor)
    ;[1 1 1] Generate Random Color
    (Rendering|Material|SetVectorParameterValue (Variables|Default|GetCarBodyMatInst) "AlbedoColor" (Utilities|Array|Get(acopy) _carcolorpalette (Math|Random|RandomInteger (Utilities|Array|Length _carcolorpalette))) :!class /Script/Engine.MaterialInstanceDynamic)
    (Rendering|Material|SetScalarParameterValue (Variables|Default|GetCarBodyMatInst) "LeafsMultiplier" (Math|Random|RandomFloatinRange 2.0 6.0) :!class /Script/Engine.MaterialInstanceDynamic)
    (Rendering|Material|SetScalarParameterValue (Variables|Default|GetCarBodyMatInst) "DamageMultiplier" (Math|Random|RandomFloatinRange 0.0 3.0) :!class /Script/Engine.MaterialInstanceDynamic)
    (else
      ;[1 1 1] Generate Color
      (Rendering|Material|SetVectorParameterValue :self (Variables|Default|GetCarBodyMatInst) :ParameterName "AlbedoColor" :!class /Script/Engine.MaterialInstanceDynamic))))

(fn ConstructCar
  (params (RunFunction :type Boolean))
  (bind _carcolorpalette (Variables|4.Colors|GetCarColorPalette))
  (bind _defaultsceneroot (Variables|Default|GetDefaultSceneRoot))
  (bind _cartype (Variables|3.MainControl|GetCarType))
  (bind _children (Components|GetChildrenComponents _defaultsceneroot false))
  (if (and RunFunction (not (Variables|1.MasterControl|GetLOCK_VALUES)))
    (Variables|1.MasterControl|SetRUN_SCRIPT false :!label _label)
    (elif (Variables|1.MasterControl|GetLOCK_VALUES)
      (Variables|1.MasterControl|SetRUN_SCRIPT false)
      (Variables|2.RandomControl|SetRandomColor false)
      (else
        (goto _label))))
  ;[1 1 1] Create Material Instance
  (bind _as프리미티브_컴포넌트 (Utilities|Casting|CastToPrimitiveComponent (Utilities|Array|Get(acopy) _children 1)))
  (bind _returnvalue (Rendering|Material|CreateDynamicMaterialInstance _as프리미티브_컴포넌트 0 (select (Variables|3.MainControl|GetCleanVersion) (Utilities|Select :Index _cartype :NewEnumerator0 "/Game/Assets/MAP_PostDistrict/Materials/Vehicles/MI_Hatchback_Clean.MI_Hatchback_Clean" :NewEnumerator1 "/Game/Assets/MAP_PostDistrict/Materials/Vehicles/MI_Pickup_Clean.MI_Pickup_Clean" :NewEnumerator2 "/Game/Assets/MAP_PostDistrict/Materials/Vehicles/MI_Wagon_Clean.MI_Wagon_Clean" :NewEnumerator3 "/Game/Assets/MAP_PostDistrict/Materials/Vehicles/MI_Ambulance_Clean.MI_Ambulance_Clean") (Utilities|Select :Index _cartype :NewEnumerator0 "/Game/Assets/MAP_PostDistrict/Materials/Vehicles/MI_Hatchback.MI_Hatchback" :NewEnumerator1 "/Game/Assets/MAP_PostDistrict/Materials/Vehicles/MI_Pickup.MI_Pickup" :NewEnumerator2 "/Game/Assets/MAP_PostDistrict/Materials/Vehicles/MI_Wagon.MI_Wagon" :NewEnumerator3 "/Game/Assets/MAP_PostDistrict/Materials/Vehicles/MI_Ambulance.MI_Ambulance")) "None" :!class /Script/Engine.PrimitiveComponent))
  (Variables|Default|SetCarBodyMatInst _returnvalue)
  ;[1 1 1] Assign Material Instance
  (for _array_element _children
    (bind _as프리미티브_컴포넌트_2 (Utilities|Casting|CastToPrimitiveComponent _array_element))
    (Rendering|Material|SetMaterial _as프리미티브_컴포넌트_2 0 (Variables|Default|GetCarBodyMatInst)))
  (if (Variables|1.MasterControl|GetLOCK_VALUES)
    _
    (else
      (Variables|4.Colors|SetActiveCarPaintColor (select (Variables|2.RandomControl|GetRandomColor) (Utilities|Array|Get(acopy) _carcolorpalette (Math|Random|RandomInteger (Utilities|Array|Length _carcolorpalette))) (Variables|4.Colors|GetActiveCarPaintColor)))))
  (Rendering|Material|SetVectorParameterValue (Variables|Default|GetCarBodyMatInst) "AlbedoColor" (Variables|4.Colors|GetActiveCarPaintColor) :!class /Script/Engine.MaterialInstanceDynamic))