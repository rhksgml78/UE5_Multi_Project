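; Spline-based wire actor that builds its wire from spline mesh components in the construction script.
; SplineMeshVar lays segments either between spline points or at fixed Spacing along the length with scaled direction tangents.
; WireVar selects one of six component variants and whether one or two material slots are set.
; Each segment gets uniform WireSize scaling and dynamic MI_Wire instances driven by color, dirt, specular, roughness and TextureVar texture sets.
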(fn ConstructionScript
  (|Wire))